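; BP_Map procedurally generates terrain around the player character, re-checking on a looping timer for grid tiles not yet built.
; Each new tile is recorded in TileGeneration and becomes a TerrainMesh section with collision and M_automatic, with height from two layers of multiplied 1D Perlin noise.
; Tiles are built with a one-vertex border for calculating normals and tangents, which GetSubSection then trims so shading can match across seams.
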(event `self.ReceiveBeginPlay`
  (`self.SpawnTilesAroundCamera`)
  (`KismetSystemLibrary.K2_SetTimer` null "SpawnTilesAroundCamera" 0.2 true))

(event `SpawnTilesAroundCamera`
  (bind (_xstart _xend _ystart _yend) (`self.GetTilesAroundPlayer`))
  (for _index (range _ystart (+ _yend 1))
    (for _index_2 (range _xstart (+ _xend 1))
      (`self.GenerateMap` _index_2 _index))))

(fn `GenerateMap`
  (params (XSectionIdex :type Integer) (YSectionIdex :type Integer))
  (locals (Vertices :type "Array of Vector Structure") (Triangles :type "Array of Integer") (UVS :type "Array of Vector2D Structure") (Offset :type "Vector Structure"))
  (bind _cellsize (`self.CellSize`))
  (bind _tilegeneration (`self.TileGeneration`))
  (bind _xvertexcount (`self.XvertexCount`))
  (bind _triangles (`local.Triangles`))
  (bind _triangles_2 (`local.Triangles`))
  (bind _section_index (`self.Section Index`))
  (bind (_offset_x _offset_y) (`KismetMathLibrary.BreakVector` (`local.Offset`)))
  (bind _cellsize_2 (`self.CellSize`))
  ;[1 1 1] Generate Vertices/UVs
  (if (not (`.ReturnValue` (`BlueprintMapLibrary.Map_Find` _tilegeneration (make `IntPoint` XSectionIdex YSectionIdex))))
    (`BlueprintMapLibrary.Map_Add` _tilegeneration (make `IntPoint` XSectionIdex YSectionIdex) (`self.Section Index`))
    (set `local.Offset` (`KismetMathLibrary.MakeVector` (`KismetMathLibrary.Conv_IntToDouble` (* (`local.XSectionIdex`) (* (- (`self.XvertexCount`) 1) _cellsize))) (`KismetMathLibrary.Conv_IntToDouble` (* (`local.YSectionIdex`) (* (- (`self.YvertexCount`) 1) _cellsize)))))
    (for _index (range -1 (+ (`self.YvertexCount`) 1))
      (for _index_2 (range -1 (+ (`self.XvertexCount`) 1))
        (bind _returnvalue (+ _offset_x (* _index_2 _cellsize_2)))
        (bind _returnvalue_2 (+ _offset_y (* _index _cellsize_2)))
        (`KismetArrayLibrary.Array_Add` (`local.Vertices`) (`KismetMathLibrary.MakeVector` _returnvalue _returnvalue_2 (`self.Height` _returnvalue _returnvalue_2)))
        (`KismetArrayLibrary.Array_Add` (`local.UVS`) (`KismetMathLibrary.MakeVector2D` (* (`KismetMathLibrary.Conv_IntToDouble` (+ _index_2 (* (`local.XSectionIdex`) (- (`self.XvertexCount`) 1)))) 1.0) (* (`KismetMathLibrary.Conv_IntToDouble` (+ _index (* (`local.YSectionIdex`) (- (`self.YvertexCount`) 1)))) 1.0)))))
    ;[1 1 1] Triangle calucation
    (for _index_3 (range (+ (`self.YvertexCount`) 1))
      (for _index_4 (range (+ (`self.XvertexCount`) 1))
        (bind _returnvalue_3 (+ _index_4 (* _index_3 _xvertexcount)))
        (`KismetArrayLibrary.Array_Add` _triangles _returnvalue_3)
        (bind _returnvalue_4 (+ _returnvalue_3 (+ _xvertexcount 2)))
        (`KismetArrayLibrary.Array_Add` _triangles _returnvalue_4)
        (bind _returnvalue_5 (+ _returnvalue_3 1))
        (`KismetArrayLibrary.Array_Add` _triangles _returnvalue_5)
        (`KismetArrayLibrary.Array_Add` _triangles_2 _returnvalue_4)
        (`KismetArrayLibrary.Array_Add` _triangles_2 (+ _returnvalue_4 1))
        (`KismetArrayLibrary.Array_Add` _triangles_2 _returnvalue_5)))
    (bind (_outvertices _outtriangles _outnormals _outuvs _outtangents) (`self.GetSubSection` (`local.Vertices`) (`local.Triangles`) (`local.UVS`)))
    (`ProceduralMeshComponent.CreateMeshSection_LinearColor` :`self` (`self.TerrainMesh`) :`SectionIndex` _section_index :`Vertices` _outvertices :`Triangles` _outtriangles :`Normals` _outnormals :`UV0` _outuvs :`Tangents` _outtangents :`bCreateCollision` true)
    (`PrimitiveComponent.SetMaterial` (`self.TerrainMesh`) _section_index "/Game/MapGeneration/material/M_automatic.M_automatic")
    (`/Engine/EditorBlueprintResources/StandardMacros.IncrementInt` (`self.Section Index`))))

(fn `GetPlayerPositionID`
  (returns (PlayerX :type Integer) (PlayerY :type Integer))
  (bind _returnvalue (`GameplayStatics.GetPlayerCharacter` 0))
  (bind _cellsize (`self.CellSize`))
  (bind (_returnvalue_x _returnvalue_y) (`KismetMathLibrary.BreakVector` (`self.K2_GetActorLocation` _returnvalue)))
  (`/Engine/EditorBlueprintResources/StandardMacros.IsValid` _returnvalue
    (:`Is Valid`
      (return (`KismetMathLibrary.FTrunc` (/ _returnvalue_x (* _cellsize (- (`self.XvertexCount`) 1)))) (`KismetMathLibrary.FTrunc` (/ _returnvalue_y (* _cellsize (- (`self.YvertexCount`) 1))))))
    (:`Is Not Valid`
      (return 0 0))))

(fn `GetSubSection`
  (params (inVertices2 :type "Array of Vector Structure (by ref)") (inTriangles2 :type "Array of Integer (by ref)") (inUVs2 :type "Array of Vector2D Structure (by ref)"))
  (returns (OutVertices :type "Array of Vector Structure") (OutTriangles :type "Array of Integer") (OutNormals :type "Array of Vector Structure") (OutUVS :type "Array of Vector2D Structure") (OutTangents :type "Array of ProcMeshTangent Structure"))
  (locals (OVertices :type "Array of Vector Structure") (OTriangles :type "Array of Integer") (OUvs :type "Array of Vector2D Structure") (ONormals :type "Array of Vector Structure") (OTangents :type "Array of ProcMeshTangent Structure") (LargeNormals :type "Array of Vector Structure") (LargeTangents :type "Array of ProcMeshTangent Structure") (Idex :type Integer :default 0))
  (bind _xvertexcount (`self.XvertexCount`))
  (bind _otriangles (`local.OTriangles`))
  (bind _otriangles_2 (`local.OTriangles`))
  (bind (_normals _tangents) (`KismetProceduralMeshLibrary.CalculateTangentsForMesh` inVertices2 inTriangles2 inUVs2))
  (set `local.LargeNormals` _normals)
  (set `local.LargeTangents` _tangents)
  (for _index (range -1 (+ (`self.YvertexCount`) 1))
    (for _index_2 (range -1 (+ (`self.XvertexCount`) 1))
      (if (and (> _index_2 -1) (< _index_2 (`self.XvertexCount`)) (> _index -1) (< _index (`self.YvertexCount`)))
        (`KismetArrayLibrary.Array_Add` (`local.OVertices`) (`|GetArrayItem` (`local.inVertices2`) (`local.Idex`)))
        (`KismetArrayLibrary.Array_Add` (`local.OUvs`) (`|GetArrayItem` (`local.inUVs2`) (`local.Idex`)))
        (`KismetArrayLibrary.Array_Add` (`local.ONormals`) (`|GetArrayItem` (`local.LargeNormals`) (`local.Idex`)))
        (`KismetArrayLibrary.Array_Add` (`local.OTangents`) (`|GetArrayItem` (`local.LargeTangents`) (`local.Idex`))))
      (`/Engine/EditorBlueprintResources/StandardMacros.IncrementInt` (`local.Idex`))))
  (for _index_3 (range (+ (- (`self.YvertexCount`) 2) 1))
    (for _index_4 (range (+ (- (`self.XvertexCount`) 2) 1))
      (bind _returnvalue (+ _index_4 (* _index_3 _xvertexcount)))
      (`KismetArrayLibrary.Array_Add` _otriangles_2 _returnvalue)
      (bind _returnvalue_2 (+ _returnvalue _xvertexcount))
      (`KismetArrayLibrary.Array_Add` _otriangles_2 _returnvalue_2)
      (bind _returnvalue_3 (+ _returnvalue 1))
      (`KismetArrayLibrary.Array_Add` _otriangles_2 _returnvalue_3)
      (`KismetArrayLibrary.Array_Add` _otriangles _returnvalue_2)
      (`KismetArrayLibrary.Array_Add` _otriangles (+ _returnvalue_2 1))
      (`KismetArrayLibrary.Array_Add` _otriangles _returnvalue_3)))
  (return (`local.OVertices`) (`local.OTriangles`) (`local.ONormals`) (`local.OUvs`) (`local.OTangents`)))

(fn `GetTilesAroundPlayer`
  (returns (Xstart :type Integer) (Xend :type Integer) (Ystart :type Integer) (Yend :type Integer))
  (bind (_playerx _playery) (`self.GetPlayerPositionID`))
  (bind _numsectionx (`self.NumSectionX`))
  (bind _numsectiony (`self.NumSectionY`))
  (bind _returnvalue (- _playerx (/ _numsectionx 2)))
  (bind _returnvalue_2 (- _playery (/ _numsectiony 2)))
  (return _returnvalue (+ _returnvalue _numsectionx -1) _returnvalue_2 (+ _returnvalue_2 _numsectiony -1)))

(fn `Height`
  (params (inX :type "Float (double-precision)") (inY :type "Float (double-precision)"))
  (returns (ReturnValue :type "Float (double-precision)"))
  (return (+ (`self.PerlinNoise2D` inX inY 0.0001 10000.0) (`self.PerlinNoise2D` inX inY 0.001 500.0))))

(fn `PerlinNoise2D`
  (params (X :type "Float (double-precision)") (Y :type "Float (double-precision)") (Scale :type "Float (double-precision)") (AMP :type "Float (double-precision)"))
  (returns (ReturnValue :type "Float (double-precision)"))
  (return (* (* (`KismetMathLibrary.PerlinNoise1D` (+ (* X Scale) 0.1)) (`KismetMathLibrary.PerlinNoise1D` (+ (* Y Scale) 0.1))) AMP)))

(fn `UserConstructionScript`)